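; BP_DestructibleActor is a breakable prop that shatters in two stages when hit and then removes itself.
; OnGetHit clears the actor's tags and applies radius damage to the main destructible component at the hit location, disabling its collision.
; After a short delay, the secondary destructible component loses collision and breaks from its own center.
; The actor destroys itself a few seconds later.
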(event EventBeginPlay)

(event Collision|EventActorBeginOverlap
  (params (OtherActor :type Actor%20Object%20Reference)))

(event EventTick
  (params (DeltaSeconds :type Float%20%28single-precision%29)))

(event EventOnGetHit
  (params (GetHitLocation :type Vector :default "0, 0, 0") (ImpulseDir :type Vector :default "0, 0, 0"))
  (bind _otherdestructiblecomponent (Variables|Default|GetOtherDestructibleComponent))
  (bind _maindestructiblecomponent (Variables|Default|GetMainDestructibleComponent))
  (Utilities|Array|Clear (Variables|Default|GetTags))
  (Class|DestructibleComponent|ApplyRadiusDamage _maindestructiblecomponent 1e+02 GetHitLocation 0.0 1e+02 true)
  (Collision|SetCollisionEnabled _maindestructiblecomponent "NoCollision")
  (Utilities|FlowControl|Delay 0.5)
  (Collision|SetCollisionEnabled _otherdestructiblecomponent "NoCollision")
  (Class|DestructibleComponent|ApplyRadiusDamage _otherdestructiblecomponent 1e+02 (Transformation|GetWorldLocation _otherdestructiblecomponent) 0.0 1e+02 true)
  (Utilities|FlowControl|Delay 5.0)
  (Actor|DestroyActor))

(fn ConstructionScript)