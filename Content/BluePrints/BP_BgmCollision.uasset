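; BP_BgmCollision is a trigger actor that starts background music when something enters its sphere and stops it when the game ends.
; The sphere's overlap fades the Audio component in, then disables its own collision so it fires only once.
; On BeginPlay it binds to the CombatGameMode game-over delegate, which fades the audio out linearly.
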(event OnComponentBeginOverlap(Sphere)
  (params (OverlappedComponent :type Primitive%20Component%20Object%20Reference) (OtherActor :type Actor%20Object%20Reference) (OtherComp :type Primitive%20Component%20Object%20Reference) (OtherBodyIndex :type Integer) (bFromSweep :type Boolean) (SweepResult :type Hit%20Result%20Structure%20%28by%20ref%29))
  (Audio|Components|Audio|FadeIn (Variables|Default|GetAudio) 5.0 1.0 0.0 "Linear" :!class /Script/Engine.AudioComponent)
  (Collision|SetCollisionEnabled (Variables|Default|GetSphere) "NoCollision"))

(event Custom|OnGameOver
  (Audio|Components|Audio|FadeOut (Variables|Default|GetAudio) 5.0 0.0 "Linear" :!class /Script/Engine.AudioComponent))

(event EventBeginPlay
  (bind _ascombat_game_mode (Utilities|Casting|CastToCombatGameMode (Game|GetGameMode)))
  (bind _output_get (Variables|Default|SetCombat%20Game%20Mode _ascombat_game_mode))
  (EventDispatchers|AssignOnGameOverDelegate _output_get (delegate Custom|OnGameOver)))

(event Collision|EventActorBeginOverlap
  (params (OtherActor :type Actor%20Object%20Reference)))

(event EventTick
  (params (DeltaSeconds :type Float%20%28single-precision%29)))

(fn ConstructionScript)